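; Fireball projectile actor with a Paper2D flipbook visual that damages what it overlaps, apart from the player character class MyCharacter.
; The construction script adds the flipbook, and BeginPlay attaches a fireball trail emitter.
; On overlap with any actor that fails the MyCharacter cast, it sends OnDamageMessage to that actor, spawns an ExplodyPuff at its own location and destroys itself.
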(event EventBeginPlay
  (Development|PrintString "Create Proyectile")
  (Effects|SpawnEmitterAttached "/Game/Effects/FireballTrail.FireballTrail" (Variables|Default|GetTrailAttach) "None" "0, 0, 0" "0, 0, 0" "1.000000,1.000000,1.000000" "SnapToTarget"))

(event Collision|EventActorBeginOverlap
  (params (OtherActor :type Actor%20Object%20Reference))
  (Utilities|Casting|CastToMyCharacter OtherActor
    (:CastFailed
      (Class|IDamageEnemys|OnDamage(Message) OtherActor)
      (Development|PrintString "Enemy collision Succeful")
      (Game|SpawnActorfromClass "/Game/Blueprints/ExplodyPuff.ExplodyPuff_C" (Math|Conversions|ToTransform(Vector) (Transformation|GetActorLocation)) "AdjustIfPossibleButDontSpawnIfColliding" "OverrideRootScale" 0 0)
      (Actor|DestroyActor))))

(fn ConstructionScript
  (AddComponent|AddPaperFlipbookComponent false (Math|Transform|MakeTransform "-30.000000, 0,5.000000" "0, 0, 0" "1.500000,1.500000,1.500000")))